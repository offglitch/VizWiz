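; BP_CustomSkybox_1 is a skybox Blueprint that animates a rotating sky on its SkySphere mesh.
; The construction script creates a dynamic material instance from SkyMaterial and assigns it to the sphere's first material slot.
; Each tick reads that instance's "Angle" parameter and advances it by RotationSpeed scaled by delta time, driving the rotation through the material instead of the mesh transform.
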(event `self.ReceiveTick`
  (params (DeltaSeconds :type "Float (single-precision)"))
  (bind _asmaterial_instance_dynamic (cast `MaterialInstanceDynamic` (`PrimitiveComponent.GetMaterial` (`self.SkySphere`) 0)))
  (bind _returnvalue (`MaterialInstanceDynamic.K2_GetScalarParameterValue` _asmaterial_instance_dynamic "Angle"))
  (`MaterialInstanceDynamic.SetScalarParameterValue` _asmaterial_instance_dynamic "Angle" (+ _returnvalue (* DeltaSeconds (`self.RotationSpeed`)))))

(fn `UserConstructionScript`
  (bind _returnvalue (`KismetMaterialLibrary.CreateDynamicMaterialInstance` (`self.SkyMaterial`)))
  (`PrimitiveComponent.SetMaterial` (`self.SkySphere`) 0 _returnvalue))